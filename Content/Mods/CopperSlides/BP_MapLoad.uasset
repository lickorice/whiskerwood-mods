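; Mod map-load actor for CopperSlides that gives slide buildings a copper metal tube look.
; On BeginPlay it binds to the mod API's loading-finished and building-spawned events.
; When loading finishes it swaps the first material of every existing Slide's mesh, and newly spawned slides get the same swap.
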(event Custom|OnLoadingFinished
  (bind _outactors (Actor|GetAllActorsOfClass "/Game/GridActors/Slide.Slide_C"))
  (for _array_element _outactors
    (bind _asslide (Utilities|Casting|CastToSlide _array_element))
    (Rendering|Material|SetMaterial (Variables|/Game/GridActors/Slide.Slide_C|GetStaticMesh12 _asslide) 0 "/Game/Mods/CopperSlides/MI_Copper_MetalTube.MI_Copper_MetalTube")))

(event Custom|OnSlideSpawned
  (params (Actor :type Actor%20Object%20Reference))
  (bind _asslide (Utilities|Casting|CastToSlide Actor))
  (Rendering|Material|SetMaterial (Variables|/Game/GridActors/Slide.Slide_C|GetStaticMesh12 _asslide) 0 "/Game/Mods/CopperSlides/MI_Copper_MetalTube.MI_Copper_MetalTube"))

(event EventBeginPlay
  (EventDispatchers|BindEventtoOnLoadingFinished (Class|ModAPI|GetModAPI) (delegate Custom|OnLoadingFinished))
  (EventDispatchers|BindEventtoOnBuildingSpawned (Class|ModAPI|GetModAPI) (delegate Custom|OnSlideSpawned)))

(fn ConstructionScript)