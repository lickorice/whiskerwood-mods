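; Startup Blueprint for the Short Nights mod, which offers a setting for game speed at night.
; On BeginPlay it registers the night speed multiplier option with the mod API; nothing here applies the chosen value.
; Tick is empty, and unconnected leftovers hold an older approach that wrote phase lengths to the SystemTunes DataTable, plus a debug widget showing night length.
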(event EventBeginPlay
  (Class|ModAPI|RegisterModOptions (Class|ModAPI|GetModAPI) (Variables|Default|GetNightLengthOptionId) "Short Nights: Night Speed (Multiplier)" (Variables|Default|GetOptionsValues) "2x" "Game speed when it is night time"))

(event EventTick
  (params (DeltaSeconds :type Float%20%28single-precision%29))
  ;[0.15 0.15 0.15 0.5] Temp
)

(fn ConstructionScript)