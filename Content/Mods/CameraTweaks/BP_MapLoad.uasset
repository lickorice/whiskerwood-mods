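; Map-load actor for the CameraTweaks mod that applies user options to the play pawn's camera config.
; BeginPlay finds BP_Pawn_Play, reads saved options through the mod API, widens camera distance limits and listens for option changes.
; ChangeModOptions maps each option by array index to pan speed, fast-pan multiplier, tilt limits or zoom speed.
; Tick switches between base and fast pan speed while Left Shift is held.
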(event Custom|OnOptionChanged
  (params (optionId :type String) (Value :type String))
  (Class|ModAPI|LogMessage (Class|ModAPI|GetModAPI) (Utilities|String|Append optionId Value))
  (bind (_array_element _array_index) (Utilities|Array|ForEachLoopwithBreak (Variables|Default|GetOptions) :!label _label)
    (:LoopBody
      (if (Utilities|Enum|Equal(Enum) (.OptionId (Utilities|Struct|BreakST_CameraTweaksOptions _array_element)) optionId)
        (CallFunction|ChangeModOptions _array_index Value)
        (goto _label Break)))))

(event EventBeginPlay
  (EventDispatchers|BindEventtoOnOptionChanged (Class|ModAPI|GetModAPI) (EventDispatchers|CreateEvent :!event Custom|OnOptionChanged))
  (bind _returnvalue (Actor|GetActorOfClass "/Game/Code/UnrealComponents/BP_Pawn_Play.BP_Pawn_Play_C"))
  (Variables|Default|SetPawnPlay _returnvalue)
  (for (_array_element _array_index) (Variables|Default|GetOptions)
    (bind _returnvalue_2 (Class|ModAPI|ReadModOptionValue (Class|ModAPI|GetModAPI) (.OptionId (Utilities|Struct|BreakST_CameraTweaksOptions _array_element)) (.OptionDefaultValue (Utilities|Struct|BreakST_CameraTweaksOptions _array_element))))
    (CallFunction|ChangeModOptions _array_index _returnvalue_2))
  (Utilities|Struct|SetmembersinPlayPawnCfg (Variables|/Script/ProjectArco.Pawn_Play|Getm_config (Variables|Default|GetPawnPlay)) 5e+01 5e+04))

(event EventTick
  (params (DeltaSeconds :type Float%20%28single-precision%29))
  (bind _pawnplay (Variables|Default|GetPawnPlay))
  (bind _m_config (Variables|/Script/ProjectArco.Pawn_Play|Getm_config _pawnplay))
  (Utilities|IsValid _pawnplay
    (:Is%20Valid
      (if (Game|Player|IsInputKeyDown (Game|GetPlayerController 0) "LeftShift")
        (Utilities|Struct|SetmembersinPlayPawnCfg _m_config (Variables|Default|GetFastPanSpeed))
        (else
          (Utilities|Struct|SetmembersinPlayPawnCfg _m_config (Variables|Default|GetBasePanSpeed)))))))

(fn ConstructionScript)

(fn ChangeModOptions
  (params (Index :type Integer) (Value :type String))
  (switch int Index
    (:0
      (bind _output_get (Variables|Default|SetBasePanSpeed (Math|Conversions|ToFloat(Integer) Value)))
      (Utilities|Struct|SetmembersinPlayPawnCfg (Variables|/Script/ProjectArco.Pawn_Play|Getm_config (Variables|Default|GetPawnPlay)) _output_get))
    (:1
      (Variables|Default|SetFastPanSpeed (* (Variables|Default|GetBasePanSpeed) (Math|Conversions|ToFloat(Integer) (Utilities|String|GetSubstring Value 0)))))
    (:2
      (bind _result (Math|Float|NegateFloat (Math|Conversions|ToFloat(Integer) Value))
        (:%20%20
          (Utilities|Struct|SetmembersinPlayPawnCfg (Variables|/Script/ProjectArco.Pawn_Play|Getm_config (Variables|Default|GetPawnPlay)) _result))))
    (:3
      (bind _result_2 (Math|Float|NegateFloat (Math|Conversions|ToFloat(Integer) Value))
        (:%20%20
          (Utilities|Struct|SetmembersinPlayPawnCfg (Variables|/Script/ProjectArco.Pawn_Play|Getm_config (Variables|Default|GetPawnPlay)) _result_2))))
    (:4
      (Utilities|Struct|SetmembersinPlayPawnCfg (Variables|/Script/ProjectArco.Pawn_Play|Getm_config (Variables|Default|GetPawnPlay)) (/ (Math|Conversions|ToFloat(Integer) Value) 1e+01)))))