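; Mod map-load actor for PrettierPath that restyles FastFloor stone path pieces with cobblestone visuals.
; On BeginPlay it reads the comparison option and binds to mod API events for loading finished, building spawned and option changed.
; SetMeshOrMat either swaps in the cobblestone slab mesh or uses the stone slab mesh with a cobblestone material.
; It runs on all floors after load or option change, and on each spawned one.
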(event Custom|OnLoadingFinished
  (bind _outactors (Actor|GetAllActorsOfClass "/Game/GridActors/slimActors/FastFloor.FastFloor_C"))
  (for _array_element _outactors
    (CallFunction|SetMeshorMat _array_element)))

(event Custom|OnStonePathSpawned
  (params (Actor :type Actor%20Object%20Reference))
  (CallFunction|SetMeshorMat Actor))

(event Custom|OnOptionChanged
  (params (optionId :type String) (Value :type String))
  (if (Utilities|Enum|Equal(Enum) optionId "PrettierPath-Comparison")
    (Variables|Default|SetUseNewMesh? Value)
    (bind _outactors (Actor|GetAllActorsOfClass "/Game/GridActors/slimActors/FastFloor.FastFloor_C"))
    (for _array_element _outactors
      (CallFunction|SetMeshorMat _array_element))))

(event EventBeginPlay
  (bind _returnvalue (Class|ModAPI|ReadModOptionValue (Class|ModAPI|GetModAPI) "PrettierPath-Comparison" "True"))
  (Variables|Default|SetUseNewMesh? _returnvalue)
  (EventDispatchers|BindEventtoOnLoadingFinished (Class|ModAPI|GetModAPI) (delegate Custom|OnLoadingFinished))
  (EventDispatchers|BindEventtoOnBuildingSpawned (Class|ModAPI|GetModAPI) (delegate Custom|OnStonePathSpawned))
  (EventDispatchers|BindEventtoOnOptionChanged (Class|ModAPI|GetModAPI) (delegate Custom|OnOptionChanged)))

(fn ConstructionScript)

(fn SetMeshorMat
  (params (Object :type Object%20Object%20Reference))
  (bind _asfast_floor (Utilities|Casting|CastToFastFloor Object))
  (if (Utilities|Enum|Equal(Enum) (Variables|Default|GetUseNewMesh?) "True")
    (Components|StaticMesh|SetStaticMesh (Variables|/Game/GridActors/slimActors/FastFloor.FastFloor_C|GetSM_Bridge_Wooden_01_A3 _asfast_floor) "/Game/Mods/PrettierPath/SM_CobblestoneSlab.SM_CobblestoneSlab")
    (else
      (Components|StaticMesh|SetStaticMesh (Variables|/Game/GridActors/slimActors/FastFloor.FastFloor_C|GetSM_Bridge_Wooden_01_A3 _asfast_floor) "/Game/Assets/Meshes/Kitbash_new/SM_StoneSlab/SM_StoneSlab.SM_StoneSlab")
      (Rendering|Material|SetMaterial (Variables|/Game/GridActors/slimActors/FastFloor.FastFloor_C|GetSM_Bridge_Wooden_01_A3 _asfast_floor) 0 "/Game/Mods/PrettierPath/MI_Cobblestone.MI_Cobblestone"))))