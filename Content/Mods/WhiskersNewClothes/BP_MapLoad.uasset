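; Map-load Blueprint for the WhiskersNewClothes mod that dresses Whisker agents in woven or tailored clothing meshes matching their clothing state.
; Mod API load, spawn and option events, plus a looping timer, drive updates.
; Each agent gets one static mesh component, cached by ID and socketed to its skeleton, cleared when unclothed.
; The color option picks random or green materials; changing it forces a refresh.
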(event Custom|RefreshOnOptionChange
  (params (optionId :type String) (Value :type String))
  (if (Utilities|Enum|Equal(Enum) optionId "WhiskersNewClothes-ClothesColor")
    (bind _outactors (Actor|GetAllActorsOfClass "/Script/ProjectArco.Prototype_Agent"))
    (for _array_element _outactors
      (Utilities|FlowControl|Sequence
        (:then_0
          (CallFunction|SetWhiskerClothesonAgent _array_element "" true))))))

(event Custom|WhiskerClothesCheckInit
  (bind _outactors (Actor|GetAllActorsOfClass "/Script/ProjectArco.Prototype_Agent"))
  (for (_array_element _array_index) _outactors
    (CallFunction|SetWhiskerClothesonAgent _array_element (Utilities|String|ToString(Integer) _array_index) false)))

(event Custom|SetClothesOnWhiskerSpawn
  (params (Actor :type Actor%20Object%20Reference))
  (bind _asprototype_agent (Utilities|Casting|CastToPrototype_Agent Actor))
  (if (Variables|Default|GetLoadComplete)
    (CallFunction|SetWhiskerClothesonAgent _asprototype_agent "OnSpawn" false)))

(event EventBeginPlay
  (EventDispatchers|BindEventtoOnLoadingFinished (Class|ModAPI|GetModAPI) (delegate Custom|WhiskerClothesCheckInit))
  (EventDispatchers|BindEventtoOnWhiskerSpawned (Class|ModAPI|GetModAPI) (delegate Custom|SetClothesOnWhiskerSpawn))
  (Utilities|Time|SetTimerbyEvent (delegate Custom|WhiskerClothesCheckInit) 1e+01 true)
  (EventDispatchers|BindEventtoOnOptionChanged (Class|ModAPI|GetModAPI) (EventDispatchers|CreateEvent :!event Custom|RefreshOnOptionChange)))

(fn ConstructionScript)

(fn GetWhiskerClothes
  (params (Agent :type Prototype%20Agent%20Object%20Reference) (LogPrefix :type String))
  (bind _m_state (Variables|/Script/ProjectArco.Prototype_Agent|Getm_state Agent))
  (bind (_position _rotation _animationpositionoffset _desires _modifierstate _thoughtsstate _derived_speedpercent _derived_happiness _derived_productivity _derived_carrycapacity _isdummy _isselfticking _desirevisible _isbeingmanhandled _seekingheat _seekheatattemptcooldown _currentactiondesc _home _pathingcooldown _m_secondsuntilstarvationdeath _pollutionaverage _livepollution _lightpollutionthoughtcooldown _heavypollutionthoughtcooldown _rapidconstructioncooldown _hygiene _pendingremoval _removalreason _m_foodeatentoday _m_drinkdrunktoday _lastwanderanchor _stoodstilllastwander _lastheatstate _clothingstate) (Utilities|Struct|BreakAgentState _m_state))
  (bind _currentclothingtype (Utilities|Struct|BreakClothingState _clothingstate))
  (return (== _currentclothingtype "simpleclothes") (== _currentclothingtype "clothes") (Utilities|Enum|Equal(Enum) _currentactiondesc "whiskerActivity.home")))

(fn SetWhiskerClothesonAgent
  (params (Agent :type Prototype%20Agent%20Object%20Reference) (LogPrefix :type String) (ForceRefresh :type Boolean))
  (bind (_wovenclothes _tailoredclothes) (CallFunction|GetWhiskerClothes Agent LogPrefix))
  (bind _returnvalue (Class|ModAPI|ReadModOptionValue (Class|ModAPI|GetModAPI) "WhiskersNewClothes-ClothesColor" "Random"))
  (Utilities|FlowControl|Sequence
    (:then_0
      (if _wovenclothes
        (CallFunction|CreateorSetWhiskerClothes Agent (Variables|Default|GetMeshWoven) ForceRefresh (Utilities|Enum|Equal(Enum) _returnvalue "Random"))))
    (:then_1
      (if _tailoredclothes
        (CallFunction|CreateorSetWhiskerClothes Agent (Variables|Default|GetMeshTailored) ForceRefresh (Utilities|Enum|Equal(Enum) _returnvalue "Random"))))
    (:then_2
      (if (Math|Boolean|NORBoolean _wovenclothes _tailoredclothes)
        (CallFunction|CreateorSetWhiskerClothes Agent 0 ForceRefresh (Utilities|Enum|Equal(Enum) _returnvalue "Random"))))))

(fn SetOGHatMesh
  (params (InitialActor :type Prototype%20Agent%20Object%20Reference))
  (bind _m_hatmesh (Variables|/Script/ProjectArco.Prototype_Agent|Getm_hatMesh InitialActor))
  (bind _staticmesh (Variables|/Script/Engine.StaticMeshComponent|GetStaticMesh _m_hatmesh))
  (Utilities|FlowControl|Sequence
    (:then_0
      (if (Variables|Default|GetLoggingEnabled)
        (Class|ModAPI|LogMessage (Class|ModAPI|GetModAPI) (Utilities|String|Append "WhiskersNewClothes: [SetOGHatMesh] - Hat mesh assigned to <" (Utilities|String|ToString(Object) _staticmesh) ">"))))
    (:then_1
      (Variables|Default|SetOGHatMesh _staticmesh))))

(fn CreateorFetchWhiskerClothes
  (params (WhiskerAgent :type Prototype%20Agent%20Object%20Reference))
  (bind _m_characteristics (Variables|/Script/ProjectArco.Prototype_Agent|Getm_characteristics WhiskerAgent))
  (bind _equippedclothes (Variables|Default|GetEquippedClothes))
  (bind _id (Utilities|Struct|BreakAgentCharacteristics _m_characteristics))
  (bind (_value _returnvalue) (Utilities|Map|Find _equippedclothes _id))
  (if _returnvalue
    (return _value)
    (else
      (bind _returnvalue_2 (AddComponent|AddStaticMeshComponent WhiskerAgent false))
      (Utilities|Map|Add (Variables|Default|GetEquippedClothes) _id _returnvalue_2)
      (return _returnvalue_2))))

(fn CreateorSetWhiskerClothes
  (params (WhiskerAgent :type Prototype%20Agent%20Object%20Reference) (ClothingStaticMesh :type Static%20Mesh%20Object%20Reference) (ForceRefresh :type Boolean) (RandomizedColors :type Boolean))
  (bind _texturestailoredorwoven (Variables|Default|GetTexturesTailoredOrWoven))
  (bind (_value _returnvalue) (Utilities|Map|Find _texturestailoredorwoven ClothingStaticMesh))
  (bind (_materialinstances _staticmesh _greenmaterial _materialslotname) (Utilities|Struct|BreakWNCTexturesArray _value))
  (bind _clothesobjectreference (CallFunction|CreateorFetchWhiskerClothes WhiskerAgent))
  (if (or (!= ClothingStaticMesh (Variables|/Script/Engine.StaticMeshComponent|GetStaticMesh _clothesobjectreference)) ForceRefresh)
    (Components|StaticMesh|SetStaticMesh _clothesobjectreference ClothingStaticMesh)
    (Transformation|AttachComponentToComponent _clothesobjectreference (Variables|/Script/ProjectArco.Prototype_Agent|Getm_skeletalMesh WhiskerAgent) (Variables|Default|GetSocketName) "KeepRelative" "KeepRelative" "KeepRelative" true)
    (if _returnvalue
      (if RandomizedColors
        (Rendering|Material|SetMaterialbyName _clothesobjectreference _materialslotname (Utilities|Array|Get(acopy) _materialinstances (Math|Random|RandomIntegerinRange 0 (Utilities|Array|Length _materialinstances))))
        (else
          (Rendering|Material|SetMaterialbyName _clothesobjectreference _materialslotname _greenmaterial))))))